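; BP_TankPawn is the tank pawn Blueprint, handling the main menu and game over UI.
; Pressing Home creates a W_MainMenu2 widget and adds it to the viewport.
; When the pawn is destroyed, it creates and shows a W_GameOver widget.
; Nodes for removing those widgets and passing damage to W_HealthIndicator are unconnected and never run.
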(event Collision|EventActorBeginOverlap
  (params (OtherActor :type Actor%20Object%20Reference)))

(event EventTick
  (params (DeltaSeconds :type Float%20%28single-precision%29)))

(event EventDestroyed
  (bind _returnvalue (UserInterface|CreateWidget "/Game/Widgets/W_GameOver.W_GameOver_C"))
  (bind _output_get (Variables|Default|SetisGameOver _returnvalue))
  (UserInterface|Viewport|AddtoViewport _output_get 0))

(event Input|KeyboardEvents|Home
  (params (Key :type Key%20Structure :default "None"))
  (:Pressed
    (bind _returnvalue (UserInterface|CreateWidget "/Game/Widgets/W_MainMenu2.W_MainMenu2_C"))
    (bind _output_get (Variables|Default|SetIsOpen2 _returnvalue))
    (UserInterface|Viewport|AddtoViewport _output_get 0)))

(fn ConstructionScript)